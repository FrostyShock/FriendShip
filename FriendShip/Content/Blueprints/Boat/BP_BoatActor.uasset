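; Player-sailed boat that launches via a log roller and activates wind once four hull repair spots are fixed.
; Grabbed wheel and rope crank turn the rudder and sail; the anchor toggles wind.
; Each tick applies rudder torque, eases heading toward the wind, and feeds sail direction to BPCWind.
; Overlap volumes send ship enter/exit messages, teleport ladder users aboard, hide the ocean below deck, and report level-transition actors to GameMode.
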(event `self.ReceiveTick`
  (params (DeltaSeconds :type "Float (single-precision)"))
  (`self.Rudder Effect`)
  (`self.Wind Correct Heading`)
  (`self.Rotate Sail`)
  (`KismetSystemLibrary.PrintString` (`KismetStringLibrary.Conv_DoubleToString` (`KismetMathLibrary.VSize` (`self.GetVelocity` self))) true true (struct :`G` 0.66 :`B` 1.0 :`A` 1.0) DeltaSeconds))

(event `Get Ocean Ref`
  (bind _returnvalue (`GameplayStatics.GetActorOfClass` "/Script/Water.WaterBodyOcean"))
  (set `self.Ocean Ref` _returnvalue))

(event `self.ReceiveBeginPlay`
  (`self.Get Ocean Ref`)
  (for _array_element (`|MakeArray` (`ChildActorComponent.ChildActor` (`self.RepairSpot1`)) (`ChildActorComponent.ChildActor` (`self.RepairSpot2`)) (`ChildActorComponent.ChildActor` (`self.RepairSpot3`)) (`ChildActorComponent.ChildActor` (`self.RepairSpot4`)))
    (bind _asbp_repair_spot (cast `/Game/Blueprints/Boat/BP_RepairSpot` _array_element))
    (add `/Game/Blueprints/Boat/BP_RepairSpot.OnRepaired` _asbp_repair_spot (`|CreateDelegate` :!event `Hull Repaired`))))

(event `Hull Repaired`
  (bind _result (`/Engine/EditorBlueprintResources/StandardMacros.IncrementInt` (`self.HullSlotsFilled`))
    (:`  `
      (if (>= _result 4)
        (`/Game/Blueprints/Components/BPC_Wind.Toggle Wind Active` (`self.BPC_Wind`))
        (set `self.Out Of Water` false)
        (bind _returnvalue (`GameplayStatics.GetActorOfClass` "/Game/Blueprints/Boat/BP_LogRoller.BP_LogRoller_C"))
        (`/Game/Blueprints/Boat/BP_LogRoller.StartRolling` _returnvalue)))))

(event `/Game/Data/Interfaces/BPI_PlayerInteraction.Ship Steer`
  (params (`Input Value` :type "Vector2D Structure") (`Interaction Type` :type "/Game/Data/Enums/Enum_InteractionType Enum" :default "NewEnumerator0"))
  (switch `/Game/Data/Enums/Enum_InteractionType` `Interaction Type`
    (:`NewEnumerator0`
      (`self.Steering Wheel` `Input Value`))
    (:`NewEnumerator1`
      (`self.Sail Crank` (`KismetMathLibrary.BreakVector2D` `Input Value`)))))

(event `Wind Correct Heading`
  (bind _hullcollision (`self.hullCollision`))
  ; Wind Heading
  (if (not (`self.Out Of Water`))
    (`SceneComponent.K2_SetWorldRotation` _hullcollision (`KismetMathLibrary.RInterpTo` (`SceneComponent.K2_GetComponentRotation` _hullcollision) (`KismetMathLibrary.Conv_VectorToRotator` (`/Game/Blueprints/Components/BPC_Wind.Wind Direction` (`self.BPC_Wind`))) (`GameplayStatics.GetWorldDeltaSeconds`) 0.1) false false)))

(event `Steering Wheel`
  (params (Input :type "Vector2D Structure"))
  (bind _x (`KismetMathLibrary.BreakVector2D` Input))
  (bind _rudder (`self.Rudder`))
  (bind _shipwheel (`self.shipWheel`))
  (bind (_relativerotation_roll _relativerotation_pitch _relativerotation_yaw) (`KismetMathLibrary.BreakRotator` (`SceneComponent.RelativeRotation` _rudder)))
  (bind (_relativerotation_roll_2 _relativerotation_pitch_2 _relativerotation_yaw_2) (`KismetMathLibrary.BreakRotator` (`SceneComponent.RelativeRotation` _shipwheel)))
  ; Rudder Effect
  (`SceneComponent.K2_SetRelativeRotation` _rudder (`KismetMathLibrary.MakeRotator` _relativerotation_roll _relativerotation_pitch (`KismetMathLibrary.FClamp` (+ _relativerotation_yaw _x) -60.0 60.0)) false false)
  (`SceneComponent.K2_SetRelativeRotation` _shipwheel (`KismetMathLibrary.MakeRotator` (`KismetMathLibrary.FClamp` (+ _relativerotation_roll_2 _x) -60.0 60.0) _relativerotation_pitch_2 _relativerotation_yaw_2) false false))

(event `Rudder Effect`
  (bind _rudder (`self.Rudder`))
  (bind (_relativerotation_roll _relativerotation_pitch _relativerotation_yaw) (`KismetMathLibrary.BreakRotator` (`SceneComponent.RelativeRotation` _rudder)))
  (bind (_returnvalue_x _returnvalue_y _returnvalue_z) (`KismetMathLibrary.BreakVector` (`KismetMathLibrary.LessLess_VectorRotator` (`SceneComponent.GetForwardVector` _rudder) (`SceneComponent.K2_GetComponentRotation` (`self.hullCollision`)))))
  (bind _returnvalue_x_2 (`KismetMathLibrary.BreakVector` (* (`KismetMathLibrary.MakeVector` (- _returnvalue_x 1.0) _returnvalue_y _returnvalue_z) -10000000000000.0)))
  ; Rudder Effect
  (if (not (`self.Out Of Water`))
    (`PrimitiveComponent.AddTorqueInDegrees` (`self.hullCollision`) (`KismetMathLibrary.MakeVector` 0.0 0.0 (* _returnvalue_x_2 (`KismetMathLibrary.SignOfFloat` _relativerotation_yaw))) "None" false)))

(event `self.LevelTransition.OnComponentBeginOverlap`
  (params (OverlappedComponent :type "PrimitiveComponent Object Reference") (OtherActor :type "Actor Object Reference") (OtherComp :type "PrimitiveComponent Object Reference") (OtherBodyIndex :type Integer) (bFromSweep :type Boolean) (SweepResult :type "HitResult Structure (by ref)"))
  (if (!= OtherActor self)
    (if (`KismetSystemLibrary.DoesImplementInterface` OtherActor "/Script/FriendShip.BPI_IDSubsystem")
      (bind (_boutsuccess _outinfomessage _returnvalue) (`SpawnActorsInSubLevel.GetCurrentSublevelNameFromActor` OtherActor))
      (bind _returnvalue_2 (message `BPI_IDSubsystem.GetActorID` OtherActor))
      (message `/Game/Data/Interfaces/BPI_LevelManagement.OnLevelTransition` (`GameplayStatics.GetGameMode`) (`GameplayStatics.GetObjectClass` OtherActor) (`self.GetTransform` OtherActor) (`self.GetVelocity` OtherActor) _returnvalue _returnvalue_2))))

(event `Anchor Effect`
  (`/Game/Blueprints/Components/BPC_Wind.Toggle Wind Active` (`self.BPC_Wind`)))

(event `Debug launch`
  (`/Game/Blueprints/Components/BPC_Wind.Toggle Wind Active` (`self.BPC_Wind`))
  (set `self.Out Of Water` false)
  (bind _returnvalue (`GameplayStatics.GetActorOfClass` "/Game/Blueprints/Boat/BP_LogRoller.BP_LogRoller_C"))
  (`/Game/Blueprints/Boat/BP_LogRoller.StartRolling` _returnvalue))

(event `self.Boat Bounds.OnComponentBeginOverlap`
  (params (OverlappedComponent :type "PrimitiveComponent Object Reference") (OtherActor :type "Actor Object Reference") (OtherComp :type "PrimitiveComponent Object Reference") (OtherBodyIndex :type Integer) (bFromSweep :type Boolean) (SweepResult :type "HitResult Structure (by ref)"))
  (if (== OtherActor (`GameplayStatics.GetPlayerPawn` 0))
    (`/Engine/EditorBlueprintResources/StandardMacros.IsValid` OtherActor
      (:`Is Valid`
        (message `/Game/Data/Interfaces/BPI_PlayerInteraction.OnEnterShip` OtherActor)
        (`KismetSystemLibrary.PrintString` "Hello" :!label _label)))))

(event `self.Ladder.OnComponentBeginOverlap`
  (params (OverlappedComponent :type "PrimitiveComponent Object Reference") (OtherActor :type "Actor Object Reference") (OtherComp :type "PrimitiveComponent Object Reference") (OtherBodyIndex :type Integer) (bFromSweep :type Boolean) (SweepResult :type "HitResult Structure (by ref)"))
  (bind _returnvalue (`GameplayStatics.GetPlayerPawn` 0))
  (if (== OtherActor _returnvalue)
    (`/Engine/EditorBlueprintResources/StandardMacros.IsValid` OtherActor
      (:`Is Valid`
        (message `/Game/Data/Interfaces/BPI_PlayerInteraction.OnEnterShip` _returnvalue)
        (`self.K2_SetActorLocation` _returnvalue (`SceneComponent.K2_GetComponentLocation` (`self.playerResetPoint`)) false false)
        (goto _label)))))

(event `self.Boat Bounds.OnComponentEndOverlap`
  (params (OverlappedComponent :type "PrimitiveComponent Object Reference") (OtherActor :type "Actor Object Reference") (OtherComp :type "PrimitiveComponent Object Reference") (OtherBodyIndex :type Integer))
  (message `/Game/Data/Interfaces/BPI_PlayerInteraction.OnExitShip` OtherActor))

(event `self.BelowDeck.OnComponentBeginOverlap`
  (params (OverlappedComponent :type "PrimitiveComponent Object Reference") (OtherActor :type "Actor Object Reference") (OtherComp :type "PrimitiveComponent Object Reference") (OtherBodyIndex :type Integer) (bFromSweep :type Boolean) (SweepResult :type "HitResult Structure (by ref)"))
  (bind _ocean_ref (`self.Ocean Ref`))
  (if (== OtherActor (`GameplayStatics.GetPlayerPawn` 0))
    (`/Engine/EditorBlueprintResources/StandardMacros.IsValid` _ocean_ref
      (:`Is Valid`
        (`self.SetActorHiddenInGame` _ocean_ref true)))
    (elif (`KismetSystemLibrary.DoesImplementInterface` OtherActor "/Game/Data/Interfaces/BPI_PlayerInteraction.BPI_PlayerInteraction_C")
      (message `/Game/Data/Interfaces/BPI_PlayerInteraction.OnEnterShip` OtherActor))))

(event `self.BelowDeck.OnComponentEndOverlap`
  (params (OverlappedComponent :type "PrimitiveComponent Object Reference") (OtherActor :type "Actor Object Reference") (OtherComp :type "PrimitiveComponent Object Reference") (OtherBodyIndex :type Integer))
  (bind _ocean_ref (`self.Ocean Ref`))
  (if (== OtherActor (`GameplayStatics.GetPlayerPawn` 0))
    (`/Engine/EditorBlueprintResources/StandardMacros.IsValid` _ocean_ref
      (:`Is Valid`
        (`self.SetActorHiddenInGame` _ocean_ref false)))))

(fn `On Grabbable`
  (params (`Player Actor` :type "/Game/Blueprints/Pawns/BP_PlayerPawn Object Reference") (`Target component` :type "SceneComponent Object Reference"))
  (returns (`Interaction Type` :type "/Game/Data/Enums/Enum_InteractionType Enum"))
  (if (== `Target component` (`self.shipWheel`))
    (return "NewEnumerator0")
    (elif (== `Target component` (`self.RopeCrank`))
      (return "NewEnumerator1")
      (elif (== `Target component` (`self.Anchor`))
        (`self.Anchor Effect`)
        (return "NewEnumerator3")
        (else
          (return "NewEnumerator3"))))))

(fn `Rotate Sail`
  (bind _bpc_wind (`self.BPC_Wind`))
  (set `/Game/Blueprints/Components/BPC_Wind.Sail Direction` (`SceneComponent.GetForwardVector` (`self.sailClosed`)) _bpc_wind)
  (`SceneComponent.K2_SetWorldRotation` (`self.windDIr`) (`KismetMathLibrary.Conv_VectorToRotator` (`/Game/Blueprints/Components/BPC_Wind.Wind Direction` _bpc_wind)) false false))

(fn `Sail Crank`
  (params (`Input _Y` :type "Float (double-precision)"))
  (bind _sailclosed (`self.sailClosed`))
  (bind (_relativerotation_roll _relativerotation_pitch _relativerotation_yaw) (`KismetMathLibrary.BreakRotator` (`SceneComponent.RelativeRotation` _sailclosed)))
  (`SceneComponent.K2_SetRelativeRotation` _sailclosed (`KismetMathLibrary.MakeRotator` _relativerotation_roll _relativerotation_pitch (+ _relativerotation_yaw `Input _Y`)) false false)
  (`self.Rotate Sail`))

(fn `UserConstructionScript`
  (`/Game/Blueprints/Components/BPC_Wind.Constructor` (`self.BPC_Wind`)))
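; BP_RepairSpot is a repair slot on the boat that previews and receives actors tagged "repair".
; While the slot is unfilled, an overlapping repair actor is stored and its mesh, fetched by message call, is shown on RepairMesh with a hover material.
; Ending the overlap clears the preview and reference.
; OnRepairPlaced snaps the stored actor onto the Placeholder and hides the preview; SlotFilled is not set here.
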(event `self.Overlap.OnComponentBeginOverlap`
  (params (OverlappedComponent :type "PrimitiveComponent Object Reference") (OtherActor :type "Actor Object Reference") (OtherComp :type "PrimitiveComponent Object Reference") (OtherBodyIndex :type Integer) (bFromSweep :type Boolean) (SweepResult :type "HitResult Structure (by ref)"))
  (if (and (`self.ActorHasTag` OtherActor "repair") (not (`self.slotFilled`)))
    (set `self.RepairActor` OtherActor)
    (bind _repair_item (message `/Game/Blueprints/Interfaces/BPI_ItemInteractions.onRepairOverlap` OtherActor))
    (`StaticMeshComponent.SetStaticMesh` (`self.repairMesh`) (`StaticMeshComponent.StaticMesh` (`/Game/Blueprints/Holdables/BP_PhysTest.Mesh` _repair_item)))
    (`PrimitiveComponent.SetMaterial` (`self.repairMesh`) 0 "/Game/Art/Materials/PM_HoverMat.PM_HoverMat")
    (`PrimitiveComponent.SetMaterial` (`self.repairMesh`) 0 "/Game/Art/Materials/PM_HoverMat.PM_HoverMat")))

(event `self.Overlap.OnComponentEndOverlap`
  (params (OverlappedComponent :type "PrimitiveComponent Object Reference") (OtherActor :type "Actor Object Reference") (OtherComp :type "PrimitiveComponent Object Reference") (OtherBodyIndex :type Integer))
  (if (and (`self.ActorHasTag` OtherActor "repair") (not (`self.slotFilled`)))
    (`StaticMeshComponent.SetStaticMesh` (`self.repairMesh`) null)
    (set `self.RepairActor` null)))

(event `/Game/Blueprints/Interfaces/BPI_ItemInteractions.onRepairPlaced`
  (`self.K2_AttachToComponent` (`self.RepairActor`) (`self.placeholder`) "None" "SnapToTarget" "SnapToTarget" "KeepRelative" true)
  (`StaticMeshComponent.SetStaticMesh` (`self.repairMesh`) null))

(fn `onRepairOverlap`
  (returns (`Repair Item` :type "/Game/Blueprints/Holdables/BP_RepairParent Object Reference"))
  (return null))

(fn `UserConstructionScript`)
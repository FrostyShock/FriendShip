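; Large sailable boat with a grabbable wheel and sail crank, plus an anchor that toggles wind propulsion.
; Wheel input turns a clamped rudder that torques the hull each tick, while the hull slowly interpolates toward wind heading.
; Crank input yaws the sail and updates BPCWind's sail direction.
; Bounds overlaps set the player's OnShip flag, swap out underwater post-process aboard, and send MakePersistentMessage to other interactable actors.
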(event `self.Boat Bounds.OnComponentBeginOverlap`
  (params (OverlappedComponent :type "PrimitiveComponent Object Reference") (OtherActor :type "Actor Object Reference") (OtherComp :type "PrimitiveComponent Object Reference") (OtherBodyIndex :type Integer) (bFromSweep :type Boolean) (SweepResult :type "HitResult Structure (by ref)"))
  (if (== OtherActor (`GameplayStatics.GetPlayerPawn` 0))
    (bind _asbp_player_pawn (cast `/Game/Blueprints/Pawns/BP_PlayerPawn` OtherActor))
    (set `/Game/Blueprints/Pawns/BP_PlayerPawn.OnShip` true _asbp_player_pawn)
    (`|VariableSetRef` (`.WeightedBlendables` (break `PostProcessSettings` (`CameraComponent.PostProcessSettings` (`/Game/Blueprints/Pawns/BP_PlayerPawn.Camera` _asbp_player_pawn)))) (make `WeightedBlendables` (`|MakeArray` (make `WeightedBlendable` -1.0))))
    (elif (`KismetSystemLibrary.DoesImplementInterface` OtherActor "/Game/Blueprints/Interfaces/BPI_PlayerInteraction.BPI_PlayerInteraction_C")
      (message `/Game/Blueprints/Interfaces/BPI_PlayerInteraction.Make Persistent` OtherActor))))

(event `self.ReceiveTick`
  (params (DeltaSeconds :type "Float (single-precision)"))
  (`self.Rudder Effect`)
  (`self.Wind Correct Heading`))

(event `self.Boat Bounds.OnComponentEndOverlap`
  (params (OverlappedComponent :type "PrimitiveComponent Object Reference") (OtherActor :type "Actor Object Reference") (OtherComp :type "PrimitiveComponent Object Reference") (OtherBodyIndex :type Integer))
  (if (== OtherActor (`GameplayStatics.GetPlayerPawn` 0))
    (bind _asbp_player_pawn (cast `/Game/Blueprints/Pawns/BP_PlayerPawn` OtherActor))
    (set `/Game/Blueprints/Pawns/BP_PlayerPawn.OnShip` false _asbp_player_pawn)
    (`|VariableSetRef` (`.WeightedBlendables` (break `PostProcessSettings` (`CameraComponent.PostProcessSettings` (`/Game/Blueprints/Pawns/BP_PlayerPawn.Camera` _asbp_player_pawn)))) (make `WeightedBlendables` (`|MakeArray` (make `WeightedBlendable` 1.0 "/Water/Materials/PostProcessing/MI_UnderWater_PostProcess_Volume_Custom.MI_UnderWater_PostProcess_Volume_Custom"))))))

(event `self.Ship Steer`
  (params (`Input Value` :type "Vector2D Structure") (`Interaction Type` :type "/Game/Data/Enums/Enum_InteractionType Enum" :default "NewEnumerator0"))
  (switch `/Game/Data/Enums/Enum_InteractionType` `Interaction Type`
    (:`NewEnumerator0`
      (`self.Steering Wheel` `Input Value`))
    (:`NewEnumerator1`
      (`self.Sail Crank` `Input Value`))))

(event `self.ReceiveBeginPlay`
  (`/Game/Blueprints/Components/BPC_Wind.Toggle Wind Active` (`self.BPC_Wind`))
  (`self.Rotate Sail`))

(event `Rotate Sail`
  (bind _bpc_wind (`self.BPC_Wind`))
  ; Update Sail
  (set `/Game/Blueprints/Components/BPC_Wind.Sail Direction` (`SceneComponent.GetForwardVector` (`self.sailClosed`)) _bpc_wind)
  (`SceneComponent.K2_SetWorldRotation` (`self.windDIr`) (`KismetMathLibrary.Conv_VectorToRotator` (`/Game/Blueprints/Components/BPC_Wind.Wind Direction` _bpc_wind)) false false))

(event `Wind Correct Heading`
  (bind _hullcollision (`self.hullCollision`))
  ; Wind Heading
  (`SceneComponent.K2_SetWorldRotation` _hullcollision (`KismetMathLibrary.RInterpTo` (`SceneComponent.K2_GetComponentRotation` _hullcollision) (`KismetMathLibrary.Conv_VectorToRotator` (`/Game/Blueprints/Components/BPC_Wind.Wind Direction` (`self.BPC_Wind`))) (`GameplayStatics.GetWorldDeltaSeconds`) 0.1) false false))

(event `Steering Wheel`
  (params (Input :type "Vector2D Structure"))
  (bind _x (`KismetMathLibrary.BreakVector2D` Input))
  (bind _rudder (`self.Rudder`))
  (bind _shipwheel (`self.shipWheel`))
  (bind (_relativerotation_roll _relativerotation_pitch _relativerotation_yaw) (`KismetMathLibrary.BreakRotator` (`SceneComponent.RelativeRotation` _rudder)))
  (bind (_relativerotation_roll_2 _relativerotation_pitch_2 _relativerotation_yaw_2) (`KismetMathLibrary.BreakRotator` (`SceneComponent.RelativeRotation` _shipwheel)))
  ; Rudder Effect
  (`SceneComponent.K2_SetRelativeRotation` _rudder (`KismetMathLibrary.MakeRotator` _relativerotation_roll _relativerotation_pitch (`KismetMathLibrary.FClamp` (+ _relativerotation_yaw _x) -60.0 60.0)) false false)
  (`SceneComponent.K2_SetRelativeRotation` _shipwheel (`KismetMathLibrary.MakeRotator` (`KismetMathLibrary.FClamp` (+ _relativerotation_roll_2 _x) -60.0 60.0) _relativerotation_pitch_2 _relativerotation_yaw_2) false false))

(event `Rudder Effect`
  (bind _rudder (`self.Rudder`))
  (bind (_relativerotation_roll _relativerotation_pitch _relativerotation_yaw) (`KismetMathLibrary.BreakRotator` (`SceneComponent.RelativeRotation` _rudder)))
  (bind (_returnvalue_x _returnvalue_y _returnvalue_z) (`KismetMathLibrary.BreakVector` (`KismetMathLibrary.LessLess_VectorRotator` (`SceneComponent.GetForwardVector` _rudder) (`SceneComponent.K2_GetComponentRotation` (`self.hullCollision`)))))
  (bind _returnvalue_x_2 (`KismetMathLibrary.BreakVector` (* (`KismetMathLibrary.MakeVector` (- _returnvalue_x 1.0) _returnvalue_y _returnvalue_z) -3000000000.0)))
  ; Rudder Effect
  (`PrimitiveComponent.AddTorqueInDegrees` (`self.hullCollision`) (`KismetMathLibrary.MakeVector` 0.0 0.0 (* _returnvalue_x_2 (`KismetMathLibrary.SignOfFloat` _relativerotation_yaw))) "None" false))

(event `Sail Crank`
  (params (`Input ` :type "Vector2D Structure"))
  (bind _sailclosed (`self.sailClosed`))
  (bind (_relativerotation_roll _relativerotation_pitch _relativerotation_yaw) (`KismetMathLibrary.BreakRotator` (`SceneComponent.RelativeRotation` _sailclosed)))
  (`SceneComponent.K2_SetRelativeRotation` _sailclosed (`KismetMathLibrary.MakeRotator` _relativerotation_roll _relativerotation_pitch (+ _relativerotation_yaw `Input _Y`)) false false)
  (`self.Rotate Sail`))

(event `Anchor Effect`
  (`/Game/Blueprints/Components/BPC_Wind.Toggle Wind Active` (`self.BPC_Wind`)))

(fn `On Grabbable`
  (params (Actor :type "Actor Object Reference") (`Player Component` :type "SceneComponent Object Reference") (`Hit Component` :type "SceneComponent Object Reference"))
  (returns (`Interaction Type` :type "/Game/Data/Enums/Enum_InteractionType Enum"))
  (if (== `Hit Component` (`self.shipWheel`))
    (return "NewEnumerator0")
    (elif (== `Hit Component` (`self.RopeCrank`))
      (return "NewEnumerator1")
      (elif (== `Hit Component` (`self.Anchor`))
        (`self.Anchor Effect`)
        (return "NewEnumerator3")
        (else
          (return "NewEnumerator3"))))))

(fn `UserConstructionScript`
  (`/Game/Blueprints/Components/BPC_Wind.Constructor` (`self.BPC_Wind`)))
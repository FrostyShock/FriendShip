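; Spline-driven bridge actor that builds a row of repeated meshes along an editable spline.
; The construction script steps along the spline at intervals of the mesh's local max X bound plus a fixed gap, placing instanced static mesh pieces aligned to its rotation.
; When Broken is set, the last piece becomes a separate static mesh component shifted sideways in local Y.
; The event graph has no runtime logic.
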(event `self.ReceiveBeginPlay`)

(fn `UserConstructionScript`
  (bind _spline (`self.Spline`))
  (bind _returnvalue (+ (.x (`.Max` (`StaticMeshComponent.GetLocalBounds` (`self.StaticMesh`)))) 50.0))
  (bind _returnvalue_2 (`KismetMathLibrary.FFloor` (/ (`SplineComponent.GetSplineLength` (`self.Spline`)) _returnvalue)))
  (for _index (range (+ _returnvalue_2 1))
    (if (`self.broken`)
      (if (== _index _returnvalue_2)
        (bind _returnvalue_3 (* _returnvalue _index))
        (bind _returnvalue_4 (`SplineComponent.GetLocationAtDistanceAlongSpline` _spline _returnvalue_3 "Local"))
        (bind _returnvalue_5 (`SplineComponent.GetRotationAtDistanceAlongSpline` _spline _returnvalue_3 "Local"))
        (`AddComponent|NODE_AddStaticMeshComponent-0` :`RelativeTransform` (`KismetMathLibrary.MakeTransform` (`KismetMathLibrary.MakeVector` (.x _returnvalue_4) (+ (.y _returnvalue_4) 50.0) (.z _returnvalue_4)) _returnvalue_5))
        (else
          (`InstancedStaticMeshComponent.AddInstance` (`self.InstancedStaticMesh`) (`KismetMathLibrary.MakeTransform` _returnvalue_4 _returnvalue_5) false :!label _label)))
      (else
        (goto _label)))))
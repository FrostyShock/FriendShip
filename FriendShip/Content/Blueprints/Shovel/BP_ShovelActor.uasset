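; BP_ShovelActor is a grabbable, stowable shovel that can send a jump message to an overlapping actor.
; Grab and stow events use FlipFlops to toggle physics and collision; dropping line-traces down to place it just above the surface hit.
; Its Box caches overlapping BPI_ItemInteractions actors and calls OnShovelJumpMessage on the cached one when a hit's impact normal points straight down.
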(event `Holding Event`
  (bind _returnvalue (`self.K2_GetActorLocation`))
  (bind _box (`self.Box`))
  (`/Engine/EditorBlueprintResources/StandardMacros.FlipFlop`
    (:`A`
      (`PrimitiveComponent.SetCollisionEnabled` _box "NoCollision")
      (`KismetSystemLibrary.PrintString` "First"))
    (:`B`
      (`PrimitiveComponent.SetSimulatePhysics` (`self.RootMesh`) false)
      (`PrimitiveComponent.SetCollisionEnabled` _box "QueryAndPhysics")
      (`KismetSystemLibrary.PrintString` "Dropped")
      (bind _outhit (`KismetSystemLibrary.LineTraceSingle` _returnvalue (+ _returnvalue (* (`self.GetActorUpVector`) -1.0 1000.0)) "TraceTypeQuery1"))
      (bind (_bblockinghit _binitialoverlap _time _distance _location _impactpoint) (`GameplayStatics.BreakHitResult` _outhit))
      (if _bblockinghit
        (`self.K2_SetActorLocation` self (`KismetMathLibrary.MakeVector` (.x _impactpoint) (.y _impactpoint) (+ (.z _impactpoint) 50.0)) false false)))))

(event `/Game/Data/Interfaces/BPI_PlayerInteraction.OnStow`
  (bind _rootmesh (`self.RootMesh`))
  (bind _rootmesh_2 (`self.RootMesh`))
  (`/Engine/EditorBlueprintResources/StandardMacros.FlipFlop`
    (:`A`
      (`PrimitiveComponent.SetSimulatePhysics` _rootmesh_2 false)
      (`PrimitiveComponent.SetCollisionEnabled` _rootmesh_2 "NoCollision")
      (`PrimitiveComponent.SetCollisionEnabled` (`self.Box`) "NoCollision")
      (`KismetSystemLibrary.PrintString` "Stowed"))
    (:`B`
      (`self.K2_SetActorRotation` (struct))
      (`PrimitiveComponent.SetCollisionEnabled` _rootmesh "QueryAndPhysics")
      (`PrimitiveComponent.SetSimulatePhysics` _rootmesh true)
      (`KismetSystemLibrary.PrintString` "UnStowed"))))

(event `self.Box.OnComponentBeginOverlap`
  (params (OverlappedComponent :type "PrimitiveComponent Object Reference") (OtherActor :type "Actor Object Reference") (OtherComp :type "PrimitiveComponent Object Reference") (OtherBodyIndex :type Integer) (bFromSweep :type Boolean) (SweepResult :type "HitResult Structure (by ref)"))
  (if (`KismetSystemLibrary.DoesImplementInterface` OtherActor "/Game/Data/Interfaces/BPI_ItemInteractions.BPI_ItemInteractions_C")
    (set `self.Interactible Ref` OtherActor)))

(event `self.Box.OnComponentEndOverlap`
  (params (OverlappedComponent :type "PrimitiveComponent Object Reference") (OtherActor :type "Actor Object Reference") (OtherComp :type "PrimitiveComponent Object Reference") (OtherBodyIndex :type Integer))
  (if (== OtherActor (`self.Interactible Ref`))
    (set `self.Interactible Ref` null)))

(event `self.Box.OnComponentHit`
  (params (HitComponent :type "PrimitiveComponent Object Reference") (OtherActor :type "Actor Object Reference") (OtherComp :type "PrimitiveComponent Object Reference") (NormalImpulse :type "Vector Structure") (Hit :type "HitResult Structure (by ref)"))
  (if (`KismetMathLibrary.NearlyEqual_FloatFloat` (.z (`.ImpactNormal` (`GameplayStatics.BreakHitResult` Hit))) -1.0)
    (message `/Game/Data/Interfaces/BPI_ItemInteractions.On Shovel Jump` (`self.Interactible Ref`))))

(fn `On Grabbable`
  (params (`Player Actor` :type "/Game/Blueprints/Pawns/BP_PlayerPawn Object Reference") (`Target component` :type "SceneComponent Object Reference"))
  (returns (`Interaction Type` :type "/Game/Data/Enums/Enum_InteractionType Enum"))
  (`self.Holding Event`)
  (return "NewEnumerator2"))

(fn `UserConstructionScript`)
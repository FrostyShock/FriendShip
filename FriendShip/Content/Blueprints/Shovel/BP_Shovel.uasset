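; BP_Shovel is a grabbable shovel that forwards a jump message to the interactible it overlaps.
; OnGrabbable toggles the Cube's collision via FlipFlop, off first, then back on with a downward trace that snaps the shovel just above the surface below.
; Cube overlaps store or clear the BPI_ItemInteractions actor, and a hit with a straight-down normal calls OnShovelJumpMessage on it.
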(event `self.ReceiveHit`
  (params (MyComp :type "PrimitiveComponent Object Reference") (Other :type "Actor Object Reference") (OtherComp :type "PrimitiveComponent Object Reference") (bSelfMoved :type Boolean) (HitLocation :type "Vector Structure") (HitNormal :type "Vector Structure") (NormalImpulse :type "Vector Structure") (Hit :type "HitResult Structure (by ref)"))
  (if (`KismetMathLibrary.NearlyEqual_FloatFloat` (.z HitNormal) -1.0)
    (message `/Game/Blueprints/Interfaces/BPI_ItemInteractions.On Shovel Jump` (`self.Interactible Ref`))))

(event `Holding Event`
  (bind _returnvalue (`self.K2_GetActorLocation`))
  (bind _cube (`self.Cube`))
  (`/Engine/EditorBlueprintResources/StandardMacros.FlipFlop`
    (:`A`
      (`PrimitiveComponent.SetCollisionEnabled` _cube "NoCollision"))
    (:`B`
      (`PrimitiveComponent.SetCollisionEnabled` _cube "QueryAndPhysics")
      (bind _outhit (`KismetSystemLibrary.LineTraceSingle` _returnvalue (+ _returnvalue (* (`self.GetActorUpVector`) -1.0 250.0)) "TraceTypeQuery1"))
      (bind (_bblockinghit _binitialoverlap _time _distance _location _impactpoint) (`GameplayStatics.BreakHitResult` _outhit))
      (if _bblockinghit
        (`self.K2_SetActorLocation` self (`KismetMathLibrary.MakeVector` (.x _impactpoint) (.y _impactpoint) (+ (.z _impactpoint) 50.0)) false false)))))

(event `self.Cube.OnComponentBeginOverlap`
  (params (OverlappedComponent :type "PrimitiveComponent Object Reference") (OtherActor :type "Actor Object Reference") (OtherComp :type "PrimitiveComponent Object Reference") (OtherBodyIndex :type Integer) (bFromSweep :type Boolean) (SweepResult :type "HitResult Structure (by ref)"))
  (if (`KismetSystemLibrary.DoesImplementInterface` OtherActor "/Game/Blueprints/Interfaces/BPI_ItemInteractions.BPI_ItemInteractions_C")
    (set `self.Interactible Ref` OtherActor)))

(event `self.Cube.OnComponentEndOverlap`
  (params (OverlappedComponent :type "PrimitiveComponent Object Reference") (OtherActor :type "Actor Object Reference") (OtherComp :type "PrimitiveComponent Object Reference") (OtherBodyIndex :type Integer))
  (if (== (`self.Interactible Ref`) OtherActor)
    (set `self.Interactible Ref` null)))

(fn `On Grabbable`
  (params (Actor :type "Actor Object Reference") (Component :type "PrimitiveComponent Object Reference"))
  (returns (`Interaction Type` :type "/Game/Data/Enums/Enum_InteractionType Enum"))
  (`self.Holding Event`)
  (return "NewEnumerator2"))

(fn `UserConstructionScript`)
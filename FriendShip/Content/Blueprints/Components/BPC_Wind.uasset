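; BPC_Wind is an actor component that pushes its owner with wind, using a sail direction to shape the force.
; It caches the owner's root static mesh and binds to the wind effect event on GM_FriendShip.
; While active, wind events project the normalized wind direction onto SailDirection, scale it by strength and WindModifier, and apply it as force.
; ToggleWindActive switches the effect on or off.
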(event `self.ReceiveBeginPlay`
  (bind _asgm_friend_ship (cast `/Game/Levels/GameMode/GM_FriendShip` (`GameplayStatics.GetGameMode`)))
  (set `self.Game Mode Ref` _asgm_friend_ship)
  (add `/Game/Levels/GameMode/GM_FriendShip.Wind Effect` _asgm_friend_ship (`|CreateDelegate` :!event `Wind Event`)))

(event `Constructor`
  (bind _rootcomponent (`Actor.RootComponent` (`self.GetOwner`)))
  (`/Engine/EditorBlueprintResources/StandardMacros.IsValid` _rootcomponent
    (:`Is Valid`
      (bind _asstatic_mesh_component (cast `StaticMeshComponent` _rootcomponent))
      (set `self.Static Mesh Target` _asstatic_mesh_component))))

(event `Wind Event`
  (params (`Wind Strength` :type "Float (double-precision)") (`Wind Direction` :type "Vector Structure"))
  (if (`self.Active`)
    (set `self.Wind Direction` (`KismetMathLibrary.Normal` `Wind Direction`))
    (bind _output_get (set `self.Total Wind Strength` (* (* `Wind Strength` (`KismetMathLibrary.ProjectVectorOnToVector` (`self.Wind Direction`) (`self.Sail Direction`))) (`self.WindModifier`))))
    (`/Engine/EditorBlueprintResources/StandardMacros.IsValid` (`self.Static Mesh Target`)
      (:`Is Valid`
        (`PrimitiveComponent.AddForce` (`self.Static Mesh Target`) _output_get "None" false)))))

(event `Toggle Wind Active`
  (if (`self.Active`)
    (set `self.Active` false)
    (else
      (set `self.Active` true))))
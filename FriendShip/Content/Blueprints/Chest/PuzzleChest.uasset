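; Puzzle chest actor that opens when a cannonball overlaps its sphere.
; Opening spawns a BP_PhysTest item without collision; a timeline rotates the lid and scales the item, then enables collision and toggles its wind component.
; A comment flags a massive lag spike at opening.
; Shovel digging is inactive: RaiseChest is empty, and the staged tilt-and-raise logic and CanDig enabling are disconnected.
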(event `self.ReceiveBeginPlay`)

(event `self.Sphere.OnComponentBeginOverlap`
  (params (OverlappedComponent :type "PrimitiveComponent Object Reference") (OtherActor :type "Actor Object Reference") (OtherComp :type "PrimitiveComponent Object Reference") (OtherBodyIndex :type Integer) (bFromSweep :type Boolean) (SweepResult :type "HitResult Structure (by ref)"))
  (`KismetSystemLibrary.IsObjectOfSoftClass` OtherActor "/Game/Blueprints/Holdables/BP_CannonBall.BP_CannonBall_C"
    (:`True`
      (`self.Open Chest`))))

(event `self.Sphere.OnComponentEndOverlap`
  (params (OverlappedComponent :type "PrimitiveComponent Object Reference") (OtherActor :type "Actor Object Reference") (OtherComp :type "PrimitiveComponent Object Reference") (OtherBodyIndex :type Integer))
  (`KismetSystemLibrary.IsObjectOfSoftClass` OtherActor "/Game/Blueprints/Shovel/BP_Shovel.BP_Shovel_C"
    (:`True`
      (set `self.canDig` false))))

(event `self.On Shovel Jump`
  (if (`self.canDig`)
    (`self.Raise Chest`)))

(event `Open Chest`
  (bind _spawnedobject (`self.SpawnedObject`))
  (bind _chesttop (`self.ChestTop`))
  (bind (_returnvalue_location _returnvalue_rotation) (`KismetMathLibrary.BreakTransform` (`SceneComponent.K2_GetComponentToWorld` (`self.itemSpawnLocation`))))
  (bind (_relativerotation_roll _relativerotation_pitch _relativerotation_yaw) (`KismetMathLibrary.BreakRotator` (`SceneComponent.RelativeRotation` _chesttop)))
  (bind _returnvalue (`|SpawnActorFromClass` "/Game/Blueprints/Holdables/BP_PhysTest.BP_PhysTest_C" (`KismetMathLibrary.MakeTransform` _returnvalue_location _returnvalue_rotation (0.1 0.1 0.1)) "AlwaysSpawn" "MultiplyWithRoot" null false null))
  (`self.SetActorEnableCollision` _returnvalue false)
  (set `self.SpawnedObject` _returnvalue)
  ;[1 0.0167 0.000146 0.5] CAUSES MASSIVE LAG SPIKE
  (bind (_direction _float_rotate _vector_scalar) (`Timeline|Opening Anim` :!via `PlayFromStart`)
    (:`Update`
      (`SceneComponent.K2_SetRelativeRotation` _chesttop (`KismetMathLibrary.MakeRotator` _float_rotate _relativerotation_pitch _relativerotation_yaw) false false)
      (`self.SetActorScale3D` (`self.SpawnedObject`) _vector_scalar))
    (:`Finished`
      (`self.SetActorEnableCollision` _spawnedobject true)
      (`/Game/Blueprints/Components/BPC_Wind.Toggle Wind Active` (`/Game/Blueprints/Holdables/BP_PhysTest.BPC_Wind` _spawnedobject)))))

(event `Raise Chest`)

(event `self.ChestBody.OnComponentHit`
  (params (HitComponent :type "PrimitiveComponent Object Reference") (OtherActor :type "Actor Object Reference") (OtherComp :type "PrimitiveComponent Object Reference") (NormalImpulse :type "Vector Structure") (Hit :type "HitResult Structure (by ref)")))

(fn `onRepairOverlap`
  (returns (`Repair Item` :type "/Game/Blueprints/Holdables/BP_RepairParent Object Reference"))
  (return null))

(fn `UserConstructionScript`)
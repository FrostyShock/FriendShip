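; BP_LevelStreamingOverlap is a trigger volume that streams a named sublevel in and out based on overlap.
; The construction script sizes its capsule from the Height and Radius variables.
; Any actor beginning overlap prints a debug "Hello" and asynchronously loads MapToStream, making it visible once loaded.
; Any actor ending overlap unloads that level without blocking, with no filtering or overlap counting.
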(event `self.ReceiveActorBeginOverlap`
  (params (OtherActor :type "Actor Object Reference"))
  (`KismetSystemLibrary.PrintString` "Hello")
  (`GameplayStatics.LoadStreamLevel` (`self.mapToStream`) true))

(event `self.ReceiveActorEndOverlap`
  (params (OtherActor :type "Actor Object Reference"))
  (`GameplayStatics.UnloadStreamLevel` (`self.mapToStream`)))

(fn `UserConstructionScript`
  (bind _capsule (`self.Capsule`))
  (`CapsuleComponent.SetCapsuleHalfHeight` _capsule (`self.Height`) true)
  (`CapsuleComponent.SetCapsuleRadius` _capsule (`self.Radius`) true))
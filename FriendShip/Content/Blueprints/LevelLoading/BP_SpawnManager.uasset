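; Level-loading spawn manager that reports "replicable" actors leaving its sphere and spawns copies of actors on request.
; It registers with the game mode on BeginPlay, then on end overlap sends it the actor's class, transform, velocity and sublevel name.
; OnSpawnCopy spawns the given class and applies the passed velocity as an acceleration-change force if its mesh simulates physics.
; The player pawn leaving disables the sphere's collision.
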(event `self.ReceiveBeginPlay`
  (message `/Game/Data/Interfaces/BPI_LevelManagement.UpdateRelevantManager` (`GameplayStatics.GetGameMode`) self))

(event `/Game/Data/Interfaces/BPI_LevelManagement.OnSpawnCopy`
  (params (`Actor Class` :type "Actor Class Reference") (Transform :type "Transform Structure") (VelocityState :type "Vector Structure") (OriginalLevel :type String))
  (bind _returnvalue (`|SpawnActorFromClass` `Actor Class` Transform "Undefined" "MultiplyWithRoot" null null))
  (bind _returnvalue_2 (`self.GetComponentByClass` _returnvalue "/Script/Engine.StaticMeshComponent"))
  (`/Engine/EditorBlueprintResources/StandardMacros.IsValid` _returnvalue_2
    (:`Is Valid`
      (if (`SceneComponent.IsSimulatingPhysics` _returnvalue_2 "None")
        (`PrimitiveComponent.AddForce` _returnvalue_2 VelocityState "None" true)))))

(event `self.ReceiveEndPlay`
  (params (EndPlayReason :type "EEndPlayReason Enum" :default "Destroyed"))
  (`KismetSystemLibrary.PrintString` "Level Unloaded"))

(event `self.Sphere.OnComponentEndOverlap`
  (params (OverlappedComponent :type "PrimitiveComponent Object Reference") (OtherActor :type "Actor Object Reference") (OtherComp :type "PrimitiveComponent Object Reference") (OtherBodyIndex :type Integer))
  (bind _returnvalue (`GameplayStatics.GetObjectClass` OtherActor))
  (if (`self.ActorHasTag` OtherActor "replicable")
    (bind (_boutsuccess _outinfomessage _returnvalue_2) (`SpawnActorsInSubLevel.GetCurrentSublevelNameFromActor` OtherActor))
    (message `/Game/Data/Interfaces/BPI_LevelManagement.OnLevelTransition` (`GameplayStatics.GetGameMode`) _returnvalue (`self.GetTransform` OtherActor) (`self.GetVelocity` OtherActor) _returnvalue_2 (struct))
    (`KismetSystemLibrary.PrintString` (`KismetSystemLibrary.GetClassDisplayName` _returnvalue) true true (struct :`G` 0.66 :`B` 1.0 :`A` 1.0) 10.0)
    (elif (== OtherActor (`GameplayStatics.GetPlayerPawn` 0))
      (`PrimitiveComponent.SetCollisionEnabled` (`self.Sphere`) "NoCollision"))))

(fn `UserConstructionScript`
  (`SphereComponent.SetSphereRadius` (`self.Sphere`) (`self.In Sphere Radius`) true))
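; BP_PlayerPawn is a player pawn that moves and looks around through Enhanced Input actions.
; IA_Move combines the actor's forward and right vectors by the input axes and feeds the result straight to CharacterMovement as an input vector.
; IA_Look drives controller yaw and pitch, with the vertical axis negated.
; The construction script is empty.
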(event `EnhancedInput|/Game/Data/Input/Default/IA_Move`
  (params (ActionValue :type "Vector2D Structure") (ElapsedSeconds :type "Float (double-precision)") (TriggeredSeconds :type "Float (double-precision)") (InputAction :type "InputAction Object Reference" :default "/Game/Data/Input/Default/IA_Move.IA_Move"))
  (bind (_x _y) (`KismetMathLibrary.BreakVector2D` ActionValue))
  (:`Triggered`
    (`PawnMovementComponent.AddInputVector` (`self.CharacterMovement`) (+ (* (`self.GetActorForwardVector` self) _y) (* (`self.GetActorRightVector` self) _x)) false)))

(event `EnhancedInput|/Game/Data/Input/Default/IA_Look`
  (params (ActionValue :type "Vector2D Structure") (ElapsedSeconds :type "Float (double-precision)") (TriggeredSeconds :type "Float (double-precision)") (InputAction :type "InputAction Object Reference" :default "/Game/Data/Input/Default/IA_Look.IA_Look"))
  (bind (_x _y) (`KismetMathLibrary.BreakVector2D` ActionValue))
  (:`Triggered`
    (`self.AddControllerPitchInput` self (* _y -1.0))
    (`self.AddControllerYawInput` self _x)))

(fn `UserConstructionScript`)
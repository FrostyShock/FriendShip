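; Physics test holdable actor that players can grab, carry, release and throw, with buoyancy and wind components.
; OnGrabbable toggles the held state: holding suspends physics, buoyancy and wind anchor and attaches to the grabbing component, while release detaches and restores them.
; OnThrow applies a mass-independent force, and MakePersistent replaces a non-persistent actor with a persistent copy that inherits velocity.
; Construction sizes the query box from mesh bounds.
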(event `Holding Event`
  (`/Engine/EditorBlueprintResources/StandardMacros.FlipFlop`
    (:`A`
      (set `self.isHeld` true))
    (:`B`
      (set `self.isHeld` false)))
  (`self.Set held`))

(event `/Game/Blueprints/Interfaces/BPI_PlayerInteraction.On Throw`
  (params (`Throwing Force` :type "Vector Structure"))
  (`PrimitiveComponent.AddForce` (`self.Mesh`) `Throwing Force` "None" true))

(event `self.ReceiveTick`
  (params (DeltaSeconds :type "Float (single-precision)")))

(event `/Game/Blueprints/Interfaces/BPI_PlayerInteraction.Make Persistent`
  (if (not (`self.persistent`))
    (bind _returnvalue (`|SpawnActorFromClass` (`GameplayStatics.GetObjectClass` self) (`self.GetTransform` self) "Undefined" "MultiplyWithRoot" null true null))
    (`PrimitiveComponent.SetSimulatePhysics` (`self.Mesh`) true)
    (`PrimitiveComponent.SetPhysicsLinearVelocity` (`/Game/Blueprints/Holdables/BP_PhysTest.Mesh` _returnvalue) (`SceneComponent.GetComponentVelocity` (`self.Mesh`)) false "None")
    (`self.K2_DestroyActor`)))

(fn `On Grabbable`
  (params (Actor :type "Actor Object Reference") (`Player Component` :type "PrimitiveComponent Object Reference") (`Hit Component` :type "PrimitiveComponent Object Reference"))
  (returns (`Interaction Type` :type "/Game/Data/Enums/Enum_InteractionType Enum"))
  (set `self.ToAttachComp` `Player Component`)
  (`self.SetOwner` Actor)
  (`self.Holding Event`)
  (return "NewEnumerator2"))

(fn `Set held`
  (if (`self.isHeld`)
    (`ActorComponent.Deactivate` (`self.Buoyancy`))
    (set `/Game/Blueprints/Components/BPC_Wind.Anchor Up` false (`self.BPC_Wind`))
    (`PrimitiveComponent.SetSimulatePhysics` (`self.Mesh`) false)
    (`PrimitiveComponent.SetCollisionEnabled` (`self.Mesh`) "NoCollision")
    (`PrimitiveComponent.SetCollisionEnabled` (`self.Box`) "QueryOnly")
    (`self.K2_AttachToComponent` (`self.ToAttachComp`) "None" "SnapToTarget" "KeepRelative" "KeepRelative")
    (else
      (`self.K2_DetachFromActor` "KeepWorld" "KeepWorld" "KeepWorld")
      (`PrimitiveComponent.SetCollisionEnabled` (`self.Mesh`) "QueryAndPhysics")
      (set `/Game/Blueprints/Components/BPC_Wind.Anchor Up` true (`self.BPC_Wind`))
      (`PrimitiveComponent.SetSimulatePhysics` (`self.Mesh`) true)
      (`ActorComponent.Activate` (`self.Buoyancy`) false)
      (set `self.ToAttachComp` null)
      (`self.SetOwner` self))))

(fn `UserConstructionScript`
  (bind _box (`self.Box`))
  (bind _returnvalue (/ (.z (`.Max` (`StaticMeshComponent.GetLocalBounds` (`self.Mesh`)))) 2.0))
  (`/Game/Blueprints/Components/BPC_Wind.Constructor` (`self.BPC_Wind`))
  (`BoxComponent.SetBoxExtent` _box (`KismetMathLibrary.MakeVector` (.x (`.Max` (`StaticMeshComponent.GetLocalBounds` (`self.Mesh`)))) (.y (`.Max` (`StaticMeshComponent.GetLocalBounds` (`self.Mesh`)))) _returnvalue) true)
  (`SceneComponent.K2_SetRelativeLocation` _box (`KismetMathLibrary.MakeVector` 0.0 0.0 _returnvalue) false false))
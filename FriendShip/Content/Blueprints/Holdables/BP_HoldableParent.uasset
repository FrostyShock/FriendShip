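; BP_HoldableParent is the base Blueprint for items players can hold, throw and bring aboard a ship.
; Throwing applies the given force to RootMesh as an acceleration change while it simulates physics, and entering a ship toggles buoyancy.
; Construction initializes the BPCWind component and sets the pontoon radius from an override, and the grab query returns a fixed enum value.
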(event `self.ReceiveTick`
  (params (DeltaSeconds :type "Float (single-precision)")))

(event `self.ReceiveBeginPlay`)

(event `/Game/Data/Interfaces/BPI_PlayerInteraction.On Throw`
  (params (`Throwing Force` :type "Vector Structure"))
  (bind _rootmesh (`self.RootMesh`))
  (if (`SceneComponent.IsSimulatingPhysics` _rootmesh "None")
    (`PrimitiveComponent.AddForce` _rootmesh `Throwing Force` "None" true)))

(event `/Game/Data/Interfaces/BPI_PlayerInteraction.OnEnterShip`
  (`self.ToggleBuoyancy`))

(fn `On Grabbable`
  (params (`Player Actor` :type "/Game/Blueprints/Pawns/BP_PlayerPawn Object Reference") (`Target component` :type "SceneComponent Object Reference"))
  (returns (`Interaction Type` :type "/Game/Data/Enums/Enum_InteractionType Enum"))
  (return "NewEnumerator2"))

(fn `UserConstructionScript`
  (`/Game/Blueprints/Components/BPC_Wind.Constructor` (`self.BPC_Wind`))
  (set `self.PontoonRadius` (`self.Pontoon Size Override`)))
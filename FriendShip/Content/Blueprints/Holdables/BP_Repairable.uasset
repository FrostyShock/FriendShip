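; BP_Repairable is a holdable item that can be placed at a BP_RepairSpot to perform a repair.
; RootMesh overlaps use a soft-class check to set or clear CanRepair and the ActiveSlot reference as it enters or leaves a spot.
; OnGrabbable fires HoldingEvent, which sends OnRepairPlacedMessage to the active slot when repair is possible.
; OnRepairOverlap returns the item itself.
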(event `self.RootMesh.OnComponentBeginOverlap`
  (params (OverlappedComponent :type "PrimitiveComponent Object Reference") (OtherActor :type "Actor Object Reference") (OtherComp :type "PrimitiveComponent Object Reference") (OtherBodyIndex :type Integer) (bFromSweep :type Boolean) (SweepResult :type "HitResult Structure (by ref)"))
  (`KismetSystemLibrary.IsObjectOfSoftClass` OtherActor "/Game/Blueprints/Boat/BP_RepairSpot.BP_RepairSpot_C"
    (:`True`
      (set `self.CanRepair` true)
      (`/Engine/EditorBlueprintResources/StandardMacros.IsValid` OtherActor
        (:`Is Valid`
          (set `self.Active Slot` OtherActor))))))

(event `self.RootMesh.OnComponentEndOverlap`
  (params (OverlappedComponent :type "PrimitiveComponent Object Reference") (OtherActor :type "Actor Object Reference") (OtherComp :type "PrimitiveComponent Object Reference") (OtherBodyIndex :type Integer))
  (`KismetSystemLibrary.IsObjectOfSoftClass` OtherActor "/Game/Blueprints/Boat/BP_RepairSpot.BP_RepairSpot_C"
    (:`True`
      (set `self.CanRepair` false)
      (`/Engine/EditorBlueprintResources/StandardMacros.IsValid` OtherActor
        (:`Is Valid`
          (set `self.Active Slot` null))))))

(event `Holding Event`
  (if (`self.CanRepair`)
    (`/Engine/EditorBlueprintResources/StandardMacros.IsValid` (`self.Active Slot`)
      (:`Is Valid`
        (message `/Game/Data/Interfaces/BPI_ItemInteractions.onRepairPlaced` (`self.Active Slot`))))))

(fn `On Grabbable`
  (params (`Player Actor` :type "/Game/Blueprints/Pawns/BP_PlayerPawn Object Reference") (`Target component` :type "SceneComponent Object Reference"))
  (returns (`Interaction Type` :type "/Game/Data/Enums/Enum_InteractionType Enum"))
  (`self.Holding Event`)
  (return "NewEnumerator2"))

(fn `onRepairOverlap`
  (returns (`Repair Item` :type "/Game/Blueprints/Holdables/BP_Repairable Object Reference"))
  (return self))

(fn `UserConstructionScript`
  (`parent.UserConstructionScript`))
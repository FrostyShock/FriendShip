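; Base holdable repair item that the player can pick up, release, throw or place into a repair slot.
; A box overlap tracks the nearby "slottable" actor, while each grab interaction flips between held and released through a FlipFlop.
; Releasing with a valid slot notifies it and locks the item as slotted, changing its interaction type and ignoring further grabs and throws.
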(event `RepairEvent`
  (bind _available_slot (`self.Available Slot`))
  (`/Engine/EditorBlueprintResources/StandardMacros.FlipFlop`
    (:`A`
      (set `self.isHeld` true)
      (`self.Set held` :!label _label)
      (`KismetSystemLibrary.PrintString` "Released"))
    (:`B`
      (set `self.isHeld` false)
      (`/Engine/EditorBlueprintResources/StandardMacros.IsValid` _available_slot
        (:`Is Valid`
          (message `/Game/Blueprints/Interfaces/BPI_ItemInteractions.onRepairPlaced` _available_slot)
          (`self.Is Slotted`))
        (:`Is Not Valid`
          (goto _label))))))

(event `Is Slotted`
  (set `self.isSlotted` true)
  (set `self.Interaction Type` "NewEnumerator3"))

(event `self.Box.OnComponentBeginOverlap`
  (params (OverlappedComponent :type "PrimitiveComponent Object Reference") (OtherActor :type "Actor Object Reference") (OtherComp :type "PrimitiveComponent Object Reference") (OtherBodyIndex :type Integer) (bFromSweep :type Boolean) (SweepResult :type "HitResult Structure (by ref)"))
  (if (`self.ActorHasTag` OtherActor "slottable")
    (set `self.Available Slot` OtherActor)
    (`KismetSystemLibrary.PrintString` "Overlapped")))

(event `self.Box.OnComponentEndOverlap`
  (params (OverlappedComponent :type "PrimitiveComponent Object Reference") (OtherActor :type "Actor Object Reference") (OtherComp :type "PrimitiveComponent Object Reference") (OtherBodyIndex :type Integer))
  (if (`self.ActorHasTag` OtherActor "slottable")
    (set `self.Available Slot` null)))

(event `/Game/Blueprints/Interfaces/BPI_PlayerInteraction.On Throw`
  (params (`Throwing Force` :type "Vector Structure"))
  (if (not (`self.isSlotted`))
    (`PrimitiveComponent.AddForce` (`self.Mesh`) `Throwing Force` "None" true)))

(fn `On Grabbable`
  (params (Actor :type "Actor Object Reference") (`Player Component` :type "PrimitiveComponent Object Reference") (`Hit Component` :type "PrimitiveComponent Object Reference"))
  (returns (`Interaction Type` :type "/Game/Data/Enums/Enum_InteractionType Enum"))
  (if (`self.isSlotted`)
    (return (`self.Interaction Type`))
    (else
      (set `self.ToAttachComp` `Player Component`)
      (`self.RepairEvent`)
      (return (`self.Interaction Type`)))))

(fn `onRepairOverlap`
  (returns (`Repair Item` :type "/Game/Blueprints/Holdables/BP_RepairParent Object Reference"))
  (return self))

(fn `UserConstructionScript`
  (`parent.UserConstructionScript`))